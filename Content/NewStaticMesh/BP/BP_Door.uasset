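; A door Blueprint that swings open when an overlap begins on its Box trigger and closes when it ends.
; The DoorAngle timeline drives the Door's relative yaw, playing forward on begin overlap and reversing on end overlap.
; When NeedAKey is set, opening requires an actor that casts to KeySystem with DoorOneHasAKey true; a KeySystem without it prints "Need a key".
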(event OnComponentBeginOverlap(Box)
  (params (OverlappedComponent :type Primitive%20Component%20Object%20Reference) (OtherActor :type Actor%20Object%20Reference) (OtherComp :type Primitive%20Component%20Object%20Reference) (OtherBodyIndex :type Integer) (bFromSweep :type Boolean) (SweepResult :type Hit%20Result%20Structure%20%28by%20ref%29))
  ;[1 1 1] Проверка, нужен ли ключ
  (if (Variables|Default|GetNeed_A_Key)
    ;[0.4143 0.5312 1] Нужен
    (bind _askey_system (Utilities|Casting|CastToKeySystem (Variables|Default|GetActor)))
    (if (Variables|/Game/NewStaticMesh/BP/KeySystem.KeySystem_C|GetDoor_One_Has_a_Key _askey_system)
      ;[1 0.765 0.2457] Не нужен
      (bind _angle (Timeline|DoorAngle Play)
        (:Update
          (Transformation|SetRelativeRotation (Variables|Default|GetDoor) (Math|Rotator|MakeRotator 0.0 0.0 _angle) false false)))
      (else
        (Development|PrintString "Need a key" true true "(R=0.441667,G=0.032692,B=0.000000,A=1.000000)" 3.0)))
    (else
      (Timeline|DoorAngle Play))))

(event OnComponentEndOverlap(Box)
  (params (OverlappedComponent :type Primitive%20Component%20Object%20Reference) (OtherActor :type Actor%20Object%20Reference) (OtherComp :type Primitive%20Component%20Object%20Reference) (OtherBodyIndex :type Integer))
  ;[1 0.765 0.2457] Не нужен
  (bind _angle (Timeline|DoorAngle Reverse)
    (:Update
      (Transformation|SetRelativeRotation (Variables|Default|GetDoor) (Math|Rotator|MakeRotator 0.0 0.0 _angle) false false))))

(fn ConstructionScript)