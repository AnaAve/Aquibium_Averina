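; BP_Gondola is a gondola actor that pushes its physics-driven static mesh upward whenever a surface is close below, producing a simple hover.
; Each tick, a short downward line trace from the mesh checks static, dynamic and physics-body objects, with debug drawing on.
; A hit applies a constant, mass-independent upward acceleration; a calculation to taper it by hit time is left unconnected.
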(event EventBeginPlay)

(event Collision|EventActorBeginOverlap
  (params (OtherActor :type Actor%20Object%20Reference)))

(event EventTick
  (params (DeltaSeconds :type Float%20%28single-precision%29))
  (bind _returnvalue (Collision|LineTraceForObjects (Transformation|GetWorldLocation (Variables|Default|GetStaticMesh)) (+ (Transformation|GetWorldLocation (Variables|Default|GetStaticMesh)) "0.000000,0.000000,-80.000000") (Utilities|Array|MakeArray "ObjectTypeQuery1" "ObjectTypeQuery2" "ObjectTypeQuery4") false 0 "ForOneFrame"))
  (if _returnvalue
    ;[1 1 1] Применяем направ-ю силу к указ-му компоненту
    (Physics|AddForce (Variables|Default|GetStaticMesh) "0, 0,1000.000000" "None" true)))

(fn ConstructionScript)