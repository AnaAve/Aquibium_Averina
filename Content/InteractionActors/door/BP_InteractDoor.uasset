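; BP_InteractDoor is an interactable swinging door that can require a key to open.
; On interact, a locked door checks the player MainCharacter's KeyComponent, then spends one key and stays unlocked, or prints a message if none is held.
; A timeline drives the door's yaw to open it and reverses when any overlap with the Box ends.
; An unconnected KeySystem key check remains in the graph and never runs.
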(event OnComponentEndOverlap(Box)
  (params (OverlappedComponent :type Primitive%20Component%20Object%20Reference) (OtherActor :type Actor%20Object%20Reference) (OtherComp :type Primitive%20Component%20Object%20Reference) (OtherBodyIndex :type Integer))
  ;[1 0.765 0.2457] Не нужен
  (bind _angle (Timeline|Timeline_0 Reverse)
    (:Update
      (Transformation|SetRelativeRotation (Variables|Default|GetDoor) (Math|Rotator|MakeRotator 0.0 0.0 _angle) false false))))

(event EventBeginPlay
  (|CallParentFunction) ; This node is disabled and will not be called.\nDrag off pins to build functionality.
)

(event Collision|EventActorBeginOverlap
  (params (OtherActor :type Actor%20Object%20Reference))
  (|CallParentFunction OtherActor) ; This node is disabled and will not be called.\nDrag off pins to build functionality.
)

(event EventTick
  (params (DeltaSeconds :type Float%20%28single-precision%29))
  (|CallParentFunction DeltaSeconds) ; This node is disabled and will not be called.\nDrag off pins to build functionality.
)

(event EventOnInteract
  ;[1 1 1] Проверка, нужен ли ключ
  (if (Variables|Default|GetNeedAKey)
    (bind _asmain_character (Utilities|Casting|CastToMainCharacter (Game|Player|GetPlayerPawn 0)))
    (if (>= (Variables|/Game/Trash/KeyComponent.KeyComponent_C|GetKeysQuantity (Variables|/Game/Characters/MainCharacter.MainCharacter_C|GetKeyComponent _asmain_character)) 1)
      ;[1 0.765 0.2457] Не нужен
      (Variables|Default|SetNeedAKey false)
      (Default|KeyDecreasing (Variables|/Game/Characters/MainCharacter.MainCharacter_C|GetKeyComponent _asmain_character) 1)
      (bind _angle (Timeline|Timeline_0 Play)
        (:Update
          (Transformation|SetRelativeRotation (Variables|Default|GetDoor) (Math|Rotator|MakeRotator 0.0 0.0 _angle) false false)))
      (else
        (Development|PrintString "Need A key")))
    (else
      (Timeline|Timeline_0 Play))))

(fn ConstructionScript
  (|CallParentFunction))