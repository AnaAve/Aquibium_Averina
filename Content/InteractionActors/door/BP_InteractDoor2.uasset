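; BP_InteractDoor2 is an interactable door that swings open, optionally gated by a key.
; On OnInteract, if NeedAKey is set, it casts an Actor reference to KeySystem and checks DoorTwoHasAKey, printing "Need a key" when that is false.
; Otherwise a timeline drives the Door's relative yaw to open it.
; Any end overlap on the Box reverses the timeline, closing the door automatically.
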(event OnComponentEndOverlap(Box)
  (params (OverlappedComponent :type Primitive%20Component%20Object%20Reference) (OtherActor :type Actor%20Object%20Reference) (OtherComp :type Primitive%20Component%20Object%20Reference) (OtherBodyIndex :type Integer))
  ;[1 0.765 0.2457] Не нужен
  (bind _angle (Timeline|Timeline_0 Reverse)
    (:Update
      (Transformation|SetRelativeRotation (Variables|Default|GetDoor) (Math|Rotator|MakeRotator 0.0 0.0 _angle) false false))))

(event EventBeginPlay
  (|CallParentFunction) ; This node is disabled and will not be called.\nDrag off pins to build functionality.
)

(event Collision|EventActorBeginOverlap
  (params (OtherActor :type Actor%20Object%20Reference))
  (|CallParentFunction OtherActor) ; This node is disabled and will not be called.\nDrag off pins to build functionality.
)

(event EventTick
  (params (DeltaSeconds :type Float%20%28single-precision%29))
  (|CallParentFunction DeltaSeconds) ; This node is disabled and will not be called.\nDrag off pins to build functionality.
)

(event EventOnInteract
  ;[1 1 1] Проверка, нужен ли ключ
  (if (Variables|Default|GetNeedAKey)
    ;[0.4143 0.5312 1] Нужен
    (bind _askey_system (Utilities|Casting|CastToKeySystem (Variables|Default|GetActor)))
    (if (Variables|/Game/InteractionActors/KeySystem.KeySystem_C|GetDoor_Two_Has_a_Key _askey_system)
      ;[1 0.765 0.2457] Не нужен
      (bind _angle (Timeline|Timeline_0 Play)
        (:Update
          (Transformation|SetRelativeRotation (Variables|Default|GetDoor) (Math|Rotator|MakeRotator 0.0 0.0 _angle) false false)))
      (else
        (Development|PrintString "Need a key" true true "(R=0.441667,G=0.032692,B=0.000000,A=1.000000)" 3.0)))
    (else
      (Timeline|Timeline_0 Play))))

(fn ConstructionScript
  (|CallParentFunction))