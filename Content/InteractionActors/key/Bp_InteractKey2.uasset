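; Interactable key pickup that grants the key for door one when the player interacts with it.
; OnInteract casts its Actor reference to KeySystem, sets DoorOneHasAKey to true, then destroys the key actor.
; Despite the Key2 asset name, it sets the door one flag.
; BeginPlay, overlap and Tick are disabled stubs.
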(event EventBeginPlay
  (|CallParentFunction) ; This node is disabled and will not be called.\nDrag off pins to build functionality.
)

(event Collision|EventActorBeginOverlap
  (params (OtherActor :type Actor%20Object%20Reference))
  (|CallParentFunction OtherActor) ; This node is disabled and will not be called.\nDrag off pins to build functionality.
)

(event EventTick
  (params (DeltaSeconds :type Float%20%28single-precision%29))
  (|CallParentFunction DeltaSeconds) ; This node is disabled and will not be called.\nDrag off pins to build functionality.
)

(event EventOnInteract
  (Variables|/Game/InteractionActors/KeySystem.KeySystem_C|SetDoor_One_Has_a_Key (.AsKey%20System (Utilities|Casting|CastToKeySystem (Variables|Default|GetActor))) true)
  (Actor|DestroyActor))

(fn ConstructionScript
  (|CallParentFunction))